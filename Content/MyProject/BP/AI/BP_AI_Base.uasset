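; BP_AI_Base is an AI enemy that turns to face the player character and attacks on sight.
; PawnSensing's OnSeePawn casts to BP_Character, snaps rotation toward it and, while CanAttack is true, spawns an actor at the Arrow1 transform.
; Any damage acts as death: it clears CanAttack, ragdolls the mesh, then destroys the capsule and finally the actor after short delays.
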(event OnSeePawn(PawnSensing)
  (params (Pawn :type Pawn%20Object%20Reference))
  (bind _asbp_character (Utilities|Casting|CastToBP_Character Pawn))
  (Transformation|SetActorRotation (Math|Rotator|FindRelativeLookatRotation (Math|Conversions|ToTransform(Vector) (Transformation|GetActorLocation)) (Transformation|GetActorLocation _asbp_character)))
  (if (Variables|Default|GetCanAttack?)
    (Game|SpawnActorfromClass "/Game/InfimaGames/FreeFPSTemplate/Core/BP_Bullet.BP_Bullet_C" (Transformation|GetWorldTransform (Variables|Default|GetArrow1)) "Undefined" "MultiplyWithRoot" 0 0)))

(event Game|Damage|EventAnyDamage
  (params (Damage :type Float%20%28single-precision%29) (DamageType :type Damage%20Type%20Object%20Reference) (InstigatedBy :type Controller%20Object%20Reference) (DamageCauser :type Actor%20Object%20Reference))
  (Variables|Default|SetCanAttack? false)
  (Physics|SetSimulatePhysics (Variables|Character|GetMesh) true)
  (Utilities|FlowControl|Delay 1.0)
  (Components|DestroyComponent (Variables|Collision|GetCapsuleComponent))
  (Utilities|FlowControl|Delay 4.0)
  (Actor|DestroyActor))

(fn ConstructionScript)